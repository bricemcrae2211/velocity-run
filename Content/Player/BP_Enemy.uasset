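; BP_Enemy is an enemy actor that can take damage and fire projectiles.
; Damageenemy subtracts damage from the AcHealth component, prints the new value for debugging and destroys the actor when health reaches zero or below.
; Shoot spawns a Bp_Projectile1 at the Scene component's world transform.
; The event graph has no active logic, nothing here calls either function, and BPlayerInRange is unused.
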(event EventBeginPlay)

(event Collision|EventActorBeginOverlap
  (params (OtherActor :type Actor%20Object%20Reference)))

(event EventTick
  (params (DeltaSeconds :type Float%20%28single-precision%29)))

(fn ConstructionScript)

(fn Damageenemy
  (params (damage :type Float%20%28double-precision%29))
  (bind _ac_health (Variables|Default|Getac_health))
  (Development|PrintString (Utilities|String|ToString(Float) (- (Variables|/Game/ac_health.ac_health_C|Gethealth _ac_health) damage)))
  (bind _output_get (Variables|/Game/ac_health.ac_health_C|Sethealth _ac_health (- (Variables|/Game/ac_health.ac_health_C|Gethealth _ac_health) damage)))
  (if (<= _output_get 0.0)
    (Actor|DestroyActor)))

(fn Shoot
  (Game|SpawnActorfromClass "/Game/Player/Bp_Projectile1.Bp_Projectile1_C" (Transformation|GetWorldTransform (Variables|Default|GetScene)) "Undefined" "MultiplyWithRoot" 0 0))