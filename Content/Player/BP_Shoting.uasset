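; BP_Shoting is a shooter actor that fires projectiles while its PlayerInRange and PlayerSameLevel flags are both true.
; Tick checks both flags, which this Blueprint only reads, then runs a one-second Delay that paces the repeated shots.
; Shoot0 spawns a Bp_Projectile1 at the world transform of the Scene component.
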(event EventBeginPlay
  (|CallParentFunction) ; This node is disabled and will not be called.\nDrag off pins to build functionality.
)

(event Collision|EventActorBeginOverlap
  (params (OtherActor :type Actor%20Object%20Reference))
  (|CallParentFunction OtherActor) ; This node is disabled and will not be called.\nDrag off pins to build functionality.
)

(event EventTick
  (params (DeltaSeconds :type Float%20%28single-precision%29))
  (if (Variables|Default|GetbPlayerInRange)
    (if (Variables|Default|GetbPlayerSameLevel)
      (Utilities|FlowControl|Delay 1.0)
      (CallFunction|Shoot0))))

(fn ConstructionScript
  (|CallParentFunction))

(fn Shoot0
  (Game|SpawnActorfromClass "/Game/Player/Bp_Projectile1.Bp_Projectile1_C" (Transformation|GetWorldTransform (Variables|Default|GetScene)) "Undefined" "MultiplyWithRoot" 0 0))