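; Enemy actor Blueprint that takes damage, dies at zero health and can leave a pickup behind.
; DamageEnemy subtracts damage from the AcHealth component with debug prints, then destroys the actor when health runs out.
; On death, a one-in-four roll calls SpawnPickup, which spawns a PickUp at the Scene component's transform and stores it in GunRef.
; The event graph has no active logic, so damage must be triggered externally.
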(event EventBeginPlay)

(event Collision|EventActorBeginOverlap
  (params (OtherActor :type Actor%20Object%20Reference)))

(event EventTick
  (params (DeltaSeconds :type Float%20%28single-precision%29)))

(fn ConstructionScript)

(fn DamageEnemy
  (params (damage :type Float%20%28double-precision%29))
  (bind _ac_health (Variables|Default|Getac_health))
  (Development|PrintString (Utilities|String|ToString(Float) (Utilities|Operators|Subtract (Variables|/Game/ac_health.ac_health_C|Gethealth _ac_health) damage)))
  (bind _output_get (Variables|/Game/ac_health.ac_health_C|Sethealth _ac_health (Utilities|Operators|Subtract (Variables|/Game/ac_health.ac_health_C|Gethealth _ac_health) damage)))
  (if (<= _output_get 0.0)
    (if (>= (Math|Random|RandomFloatinRange 0.0 1.0) 0.75)
      (Development|PrintString "spawnig and destrying objet")
      (CallFunction|SpawnPickup (Variables|Default|GetScene)))
    (Actor|DestroyActor)))

(fn SpawnPickup
  (params (self2 :type Scene%20Component%20Object%20Reference))
  (bind _returnvalue (Game|SpawnActorfromClass (Variables|Default|GetPickUp) (Transformation|GetWorldTransform self2) "Undefined" "MultiplyWithRoot" 0 0))
  (Variables|Default|SetGun%20ref _returnvalue)
  (return))