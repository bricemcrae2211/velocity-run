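; BP_EShoting is an enemy Blueprint that fires at the player by spawning BP_EnemyPRO actors at its Muzzle transform.
; Tick runs through a short Delay, which throttles calls to Shoot into a repeating fire interval.
; Shoot spawns only when PlayerInRange, PlayerSameLevel and PlayerInFront are all true; none of these flags are set in this graph.
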(event EventBeginPlay
  (|CallParentFunction) ; This node is disabled and will not be called.\nDrag off pins to build functionality.
)

(event Collision|EventActorBeginOverlap
  (params (OtherActor :type Actor%20Object%20Reference))
  (|CallParentFunction OtherActor) ; This node is disabled and will not be called.\nDrag off pins to build functionality.
)

(event EventTick
  (params (DeltaSeconds :type Float%20%28single-precision%29))
  (|CallParentFunction DeltaSeconds)
  (Utilities|FlowControl|Delay 0.2)
  (CallFunction|Shoot))

(fn ConstructionScript
  (|CallParentFunction))

(fn Shoot
  (if (Math|Boolean|ANDBoolean (Variables|Default|GetbPlayerInRange) (Variables|Default|GetbPlayerSameLevel) (Variables|Default|GetbPlayerInFront))
    (Development|PrintString "shoot" false)
    (Game|SpawnActorfromClass "/Game/Enemy/Projectile/BP_EnemyPRO.BP_EnemyPRO_C" (Transformation|GetWorldTransform (Variables|Default|GetMuzzle)) "Undefined" "MultiplyWithRoot" 0 0)))