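; BP_EDrone is an enemy drone Blueprint that runs a back-and-forth floating motion through its spring arm.
; Every Tick calls Float, which steps ARMLANGTH by a fixed amount, reverses at the UP and DOWN limits via ISGoingDown, and writes it to TargetArmLength.
; The step ignores DeltaSeconds, so speed depends on frame rate.
; Float also prints a debug "Hello" each call.
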(event EventBeginPlay
  (|CallParentFunction) ; This node is disabled and will not be called.\nDrag off pins to build functionality.
)

(event Collision|EventActorBeginOverlap
  (params (OtherActor :type Actor%20Object%20Reference))
  (|CallParentFunction OtherActor) ; This node is disabled and will not be called.\nDrag off pins to build functionality.
)

(event EventTick
  (params (DeltaSeconds :type Float%20%28single-precision%29))
  (|CallParentFunction DeltaSeconds)
  (CallFunction|Float))

(fn ConstructionScript
  (|CallParentFunction))

(fn Float
  (Development|PrintString "Hello" false)
  (if (Variables|Default|GetISGoingDown)
    (if (<= (Variables|Default|GetARMLANGTH) (Variables|Default|GetDOWN))
      (Variables|Default|SetISGoingDown false)
      (else
        (Variables|Default|SetARMLANGTH (- (Variables|Default|GetARMLANGTH) 2e+01))
        (Variables|/Script/Engine.SpringArmComponent|SetTargetArmLength (Variables|Default|GetSpringArm) (Variables|Default|GetARMLANGTH) :!label _label)
        (Development|PrintString "set" false)))
    (elif (>= (Variables|Default|GetARMLANGTH) (Variables|Default|GetUP))
      (Variables|Default|SetISGoingDown true)
      (else
        (Variables|Default|SetARMLANGTH (+ (Variables|Default|GetARMLANGTH) 2e+01))
        (goto _label)))))