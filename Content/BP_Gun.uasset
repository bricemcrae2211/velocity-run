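; BP_Gun is a gun Blueprint that acts as a skeleton for shooting and weapon stats.
; An interface shoot event passes start and end positions to OnGunShoot, which is empty here, with the end position feeding its DIRECSPEED input.
; Upgrade raises Damage by a fixed step, and getters expose Distance and FireRate.
; GetDamage returns a constant zero instead of the Damage variable.
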(event EventBeginPlay)

(event EventOnInterfaceShoot
  (params (Start%20Pos :type Vector :default "0, 0, 0") (End%20Pos :type Vector :default "0, 0, 0"))
  (CallFunction|OnGunShoot Start%20Pos End%20Pos))

(fn ConstructionScript)

(fn OnGunShoot
  (params (Start%20Pos :type Vector) (DIREC-SPEED :type Vector)))

(fn Upgrade
  (Variables|Default|SetDamage (+ (Variables|Default|GetDamage) 1e+01)))

(fn GetDamage
  (return 0.0))

(fn GetDistance
  (return (Variables|Default|GetDistance)))

(fn GetFireRate
  (return (Variables|Default|GetFireRate)))