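; BP_Missile is a missile actor that hurts the player on impact and can hurt enemies while it is held.
; A Capsule hit passes the other actor to DamagePlayer, which damages a BP_Player and then destroys the missile.
; A Capsule overlap while IsHeld is true calls DamageEnemy, which damages a BP_Enemy and leaves the missile intact.
; Both functions print the other object's name before casting.
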(event OnComponentHit(Capsule)
  (params (HitComponent :type Primitive%20Component%20Object%20Reference) (OtherActor :type Actor%20Object%20Reference) (OtherComp :type Primitive%20Component%20Object%20Reference) (NormalImpulse :type Vector :default "0, 0, 0") (Hit :type Hit%20Result%20Structure%20%28by%20ref%29))
  (CallFunction|DamagePlayer OtherActor))

(event OnComponentBeginOverlap(Capsule)
  (params (OverlappedComponent :type Primitive%20Component%20Object%20Reference) (OtherActor :type Actor%20Object%20Reference) (OtherComp :type Primitive%20Component%20Object%20Reference) (OtherBodyIndex :type Integer) (bFromSweep :type Boolean) (SweepResult :type Hit%20Result%20Structure%20%28by%20ref%29))
  (if (Variables|Default|GetIsHeld)
    (CallFunction|DamageEnemy OtherActor)))

(event EventBeginPlay)

(event Collision|EventActorBeginOverlap
  (params (OtherActor :type Actor%20Object%20Reference)))

(event EventTick
  (params (DeltaSeconds :type Float%20%28single-precision%29)))

(fn ConstructionScript)

(fn DamageEnemy
  (params (Object :type Object%20Object%20Reference))
  (Development|PrintString (Utilities|GetDisplayName Object))
  (bind _asbp_enemy (Utilities|Casting|CastToBP_Enemy Object))
  (Default|DamageEnemy _asbp_enemy 5e+01))

(fn DamagePlayer
  (params (Object :type Object%20Object%20Reference))
  (Development|PrintString (Utilities|GetDisplayName Object))
  (bind _asbp_player (Utilities|Casting|CastToBP_Player Object))
  (Default|DamagePlayer _asbp_player 25.0)
  (Actor|DestroyActor))