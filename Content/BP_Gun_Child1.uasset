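; BP_Gun_Child1 is a child gun Blueprint that fires a physical projectile.
; Its OnGunShoot override calls the parent, spawns the Projectile class at the start position and passes it the direction-speed value through BULLETSPEED.
; A disconnected line-trace damage path against enemies is left unused, and the Shoot function is empty.
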(event EventBeginPlay
  (|CallParentFunction) ; This node is disabled and will not be called.\nDrag off pins to build functionality.
)

(event Collision|EventActorBeginOverlap
  (params (OtherActor :type Actor%20Object%20Reference)))

(event EventTick
  (params (DeltaSeconds :type Float%20%28single-precision%29)))

(fn ConstructionScript)

(fn OnGunShoot
  (params (Start%20Pos :type Vector :default "0, 0, 0") (DIREC-SPEED :type Vector :default "0, 0, 0"))
  (|CallParentFunction Start%20Pos DIREC-SPEED)
  (bind _returnvalue (Game|SpawnActorfromClass "/Game/Projectile.Projectile_C" (Math|Conversions|ToTransform(Vector) Start%20Pos) "Undefined" "MultiplyWithRoot" 0 0))
  (Default|BULLETSPEED _returnvalue DIREC-SPEED))

(fn Shoot
  (params (NewParam :type Vector)))